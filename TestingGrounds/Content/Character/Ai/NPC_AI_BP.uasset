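; AI controller for guard NPCs that runs the GuardBehaviour tree on the PatrolData blackboard.
; Perception updates write a sensed actor into the blackboard enemy key and clear it on lost stimulus, ignoring actors tagged Enemy.
; Each tick sets the controlled BP_Character's Aiming flag according to whether the controller has a valid focus actor.
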(event `self.ReceiveBeginPlay`
  (bind _blackboardcomponent (`self.UseBlackboard` "/Game/Character/Ai/PatrolData.PatrolData"))
  (`self.RunBehaviorTree` "/Game/Character/Ai/GuardBehaviour.GuardBehaviour")
  (set `self.BlackBoardComp` _blackboardcomponent))

(event `self.AIPerception.OnTargetPerceptionUpdated`
  (params (Actor :type "Actor Object Reference") (Stimulus :type "AIStimulus Structure"))
  (`self.UpdateBlackBoardEnemyKey` Actor Stimulus Actor))

(event `self.ReceiveTick`
  (params (DeltaSeconds :type "Float (single-precision)"))
  (bind _asbp_character (cast `/Game/Character/Character/BP_Character` (`self.K2_GetPawn`)))
  (set `/Game/Character/Character/BP_Character.Aiming` (`KismetSystemLibrary.IsValid` (`self.GetFocusActor`)) _asbp_character))

(fn `UpdateBlackBoardEnemyKey`
  (params (ObjectValue :type "Object Object Reference") (AIStimulus :type "AIStimulus Structure (by ref)") (self2 :type "Actor Object Reference"))
  (bind _enemykey (`self.EnemyKey`))
  (bind _blackboardcomp (`self.BlackBoardComp`))
  (if (`self.ActorHasTag` self2 "Enemy")
    _
    (elif (`.bSuccessfullySensed` (break `AIStimulus` AIStimulus))
      (`BlackboardComponent.SetValueAsObject` _blackboardcomp _enemykey ObjectValue)
      (else
        (`BlackboardComponent.ClearValue` _blackboardcomp _enemykey)))))

(fn `UserConstructionScript`)